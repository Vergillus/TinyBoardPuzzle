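; Game mode for a tiny board puzzle that owns the game-over UI and the intro screen.
; On BeginPlay it creates a UI widget and an intro widget and adds both to the viewport.
; A GameOver event reveals the game-over panel, and an UpdateUI event writes the total piece number into the UI's piece counter text.
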(event EventBeginPlay
  (bind _returnvalue (UserInterface|CreateWidget "/Game/Blueprints/W_GameOver.W_GameOver_C"))
  (bind _output_get (Variables|Default|SetUI _returnvalue))
  (UserInterface|Viewport|AddtoViewport _output_get 0)
  (bind _returnvalue_2 (UserInterface|CreateWidget "/Game/Blueprints/W_Into.W_Into_C"))
  (UserInterface|Viewport|AddtoViewport _returnvalue_2 0))

(event EventTick
  (params (DeltaSeconds :type Float%20%28single-precision%29)))

(event EventGameOver
  (Widget|SetVisibility (Variables|/Game/Blueprints/W_GameOver.W_GameOver_C|GetGameOverPanel (Variables|Default|GetUI)) "Visible"))

(event EventUpdateUI
  (Rendering|Components|TextRender|SetText (Variables|/Game/Blueprints/W_GameOver.W_GameOver_C|GetPieceNumberTXT (Variables|Default|GetUI)) (Utilities|Text|ToText(Integer) (Class|TinyBoardPuzzleGameModeBase|GetTotalPieceNumber))))

(fn ConstructionScript)